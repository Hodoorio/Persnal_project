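; BP_Buildings is a building segment for the Santa running game that extends the scenery as the player advances.
; Its construction script fills six arrow-marked slots, each with one of six randomly picked child actor buildings.
; When a Player-tagged actor overlaps BoxSensor, it asks GM_RunSanta to extend the buildings.
; GetAttachPoint exposes the Arrow component's world transform as an attach point.
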(event OnComponentBeginOverlap(BoxSensor)
  (params (OverlappedComponent :type Primitive%20Component%20Object%20Reference) (OtherActor :type Actor%20Object%20Reference) (OtherComp :type Primitive%20Component%20Object%20Reference) (OtherBodyIndex :type Integer) (bFromSweep :type Boolean) (SweepResult :type Hit%20Result%20Structure%20%28by%20ref%29))
  ;[0.15 0.15 0.15 0.5] 빌딩 추가 생성
  (if (Actor|ActorHasTag OtherActor "Player")
    (bind _asgm_run_santa (Utilities|Casting|CastToGM_RunSanta (Game|GetGameMode)))
    (Default|ExtendBuildings _asgm_run_santa)))

(fn ConstructionScript
  (CallFunction|SpawnBuildings))

(fn GetAttachPoint
  (return (Transformation|GetWorldTransform (Variables|Default|GetArrow))))

(fn SpawnBuildings
  ;[0.15 0.15 0.15 0.5] 6개의 화살표의 위치에 건물 생성( 생성 처리는 함수화)
  (CallFunction|BuildProcess (Variables|Default|GetSPL1))
  (CallFunction|BuildProcess (Variables|Default|GetSPL2))
  (CallFunction|BuildProcess (Variables|Default|GetSPL3))
  (CallFunction|BuildProcess (Variables|Default|GetSPL4))
  (CallFunction|BuildProcess (Variables|Default|GetSPL5))
  (CallFunction|BuildProcess (Variables|Default|GetSPL6)))

(fn BuildProcess
  (params (SpawnArrow :type Arrow%20Component%20Object%20Reference))
  (bind _returnvalue (Transformation|GetRelativeTransform SpawnArrow))
  ;[0.15 0.15 0.15 0.5] 입력 받은 위치에 6개의 건물중에서 랜덤으로 생성
  (switch int (Math|Random|RandomIntegerinRange 0 5)
    (:0
      (AddComponent|AddChildActorComponent false _returnvalue))
    (:1
      (AddComponent|AddChildActorComponent false _returnvalue))
    (:2
      (AddComponent|AddChildActorComponent false _returnvalue))
    (:3
      (AddComponent|AddChildActorComponent false _returnvalue))
    (:4
      (AddComponent|AddChildActorComponent false _returnvalue))
    (:5
      (AddComponent|AddChildActorComponent false _returnvalue))))