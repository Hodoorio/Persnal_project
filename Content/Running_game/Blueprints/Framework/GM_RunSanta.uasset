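; GM_RunSanta is the game mode for an endless-runner Santa game, building and recycling the floor track.
; BeginPlay spawns the starting tiles and, within the same loop, reloads the saved cookie count from the CookieValue slot.
; AddFloor chains each new BP_NormalFloor to the previous tile's attach point.
; ExtendFloor adds a tile and destroys the oldest once the count exceeds the starting number plus two.
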(event EventBeginPlay
  (for _index (range 0 (- (Variables|Default|GetNumberOfTIle) 1))
    (CallFunction|AddFloor)
    (bind _returnvalue (SaveGame|LoadGamefromSlot "CookieValue"))
    (bind _assanta_save_game (Utilities|Casting|CastToSanta_SaveGame _returnvalue))
    (Variables|Default|SetCookies (Variables|/Game/Running_game/Blueprints/Framework/Santa_SaveGame.Santa_SaveGame_C|GetCookieValue _assanta_save_game))))

(fn ConstructionScript)

(fn AddFloor
  (bind _returnvalue (Game|SpawnActorfromClass "/Game/Running_game/Blueprints/Floor/BP_NormalFloor.BP_NormalFloor_C" (Variables|Default|GetFloorAttachPoint) "Undefined" "MultiplyWithRoot" 0 0))
  (bind _returnvalue_2 (Default|GetAttachPoint _returnvalue))
  (Variables|Default|SetFloorAttachPoint _returnvalue_2)
  (Utilities|Array|Add (Variables|Default|GetFloorTiles) _returnvalue))

(fn ExtendFloor
  (bind _floortiles (Variables|Default|GetFloorTiles))
  (bind _output (Utilities|Array|Get(acopy) _floortiles))
  (CallFunction|AddFloor)
  (if (> (Utilities|Array|Length (Variables|Default|GetFloorTiles)) (+ (Variables|Default|GetNumberOfTIle) 2))
    (Actor|DestroyActor _output)
    (Utilities|Array|RemoveItem _floortiles _output)))