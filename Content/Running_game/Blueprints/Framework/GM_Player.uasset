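; Game mode for a running game that builds the track from chained BP_BaseTIle actors.
; On BeginPlay it takes the first BP_BaseTIle found in the level and gives it a reference to the game mode.
; SpawnFES spawns a requested number of tiles, passing each the same reference and storing its SpawnPoint world location as the next tile's spawn location.
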(event EventBeginPlay
  (bind _outactors (Actor|GetAllActorsOfClass "/Game/Running_game/Blueprints/Floor/BP_BaseTIle.BP_BaseTIle_C"))
  (bind _output_get (Variables|Default|SetBaseTile_ref (Utilities|Array|Get(acopy) _outactors)))
  (Variables|/Game/Running_game/Blueprints/Floor/BP_BaseTIle.BP_BaseTIle_C|SetGamemode_ref _output_get self))

(fn ConstructionScript)

(fn SpawnFES
  (params (NewParam :type Integer))
  (for _index (range 0 (- NewParam 1))
    (bind _returnvalue (Game|SpawnActorfromClass "/Game/Running_game/Blueprints/Floor/BP_BaseTIle.BP_BaseTIle_C" (Math|Transform|MakeTransform (Variables|Default|GetSpawn%20Transform%20Location) "0, 0, 0" "1.000000,1.000000,1.000000") "Undefined" "MultiplyWithRoot" 0 0))
    (Variables|/Game/Running_game/Blueprints/Floor/BP_BaseTIle.BP_BaseTIle_C|SetGamemode_ref _returnvalue self)
    (Variables|Default|SetSpawn%20Transform%20Location (Transformation|GetWorldLocation (Variables|/Game/Running_game/Blueprints/Floor/BP_BaseTIle.BP_BaseTIle_C|GetSpawn_Point _returnvalue)))))