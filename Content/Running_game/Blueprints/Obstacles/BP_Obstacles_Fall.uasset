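; Falling obstacle for the running game that drops when the player approaches and kills on contact.
; BeginPlay places the mesh at BoxArrive; the player pawn entering BoxSensor restarts a timeline that lowers it toward the FallingStop marker.
; Each update lerps Z from the mesh's current height, so the motion compounds rather than following the curve directly.
; HitBox overlap passes any overlapping actor to PlayerDie.
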(event OnComponentBeginOverlap(HItBox)
  (params (OverlappedComponent :type Primitive%20Component%20Object%20Reference) (OtherActor :type Actor%20Object%20Reference) (OtherComp :type Primitive%20Component%20Object%20Reference) (OtherBodyIndex :type Integer) (bFromSweep :type Boolean) (SweepResult :type Hit%20Result%20Structure%20%28by%20ref%29))
  (CallFunction|PlayerDie OtherActor))

(event OnComponentBeginOverlap(BoxSensor)
  (params (OverlappedComponent :type Primitive%20Component%20Object%20Reference) (OtherActor :type Actor%20Object%20Reference) (OtherComp :type Primitive%20Component%20Object%20Reference) (OtherBodyIndex :type Integer) (bFromSweep :type Boolean) (SweepResult :type Hit%20Result%20Structure%20%28by%20ref%29))
  (bind _staticmesh (Variables|Default|GetStaticMesh))
  (if (== OtherActor (Game|Player|GetPlayerPawn 0))
    (bind _새_트랙_0 (Timeline|타임라인 PlayFromStart)
      (:Update
        (Transformation|SetRelativeLocation _staticmesh (Math|Vector|MakeVector 0.0 0.0 (Math|Float|Lerp (.z (Variables|/Script/Engine.SceneComponent|GetRelativeLocation _staticmesh)) (.z (Variables|/Script/Engine.SceneComponent|GetRelativeLocation (Variables|Default|GetFallingStop))) (* _새_트랙_0 0.5))) false false)))))

(event EventBeginPlay
  (|CallParentFunction)
  (Transformation|SetRelativeLocation (Variables|Default|GetStaticMesh) (Variables|Default|GetBoxArrive) false false))

(event EventTick
  (params (DeltaSeconds :type Float%20%28single-precision%29))
  (|CallParentFunction DeltaSeconds) ; 지금 이 노드는 비활성 상태입니다. \n핀을 끌어서 다른 노드를 연결하면 활성화됩니다.
)

(fn ConstructionScript
  (|CallParentFunction))