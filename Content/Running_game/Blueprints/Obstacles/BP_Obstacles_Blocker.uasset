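; BP_Obstacles_Blocker is a running-game obstacle that kills the Santa player on contact unless the player is small.
; On actor overlap it casts to BP_PlayerSanta and checks IsSmall, calling Death when that flag is false.
; After death it waits briefly and then pauses the game.
; BeginPlay, Tick and the construction script add no behavior of their own.
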(event EventBeginPlay
  (|CallParentFunction) ; 지금 이 노드는 비활성 상태입니다. \n핀을 끌어서 다른 노드를 연결하면 활성화됩니다.
)

(event Collision|EventActorBeginOverlap
  (params (OtherActor :type Actor%20Object%20Reference))
  (bind _asbp_player_santa (Utilities|Casting|CastToBP_PlayerSanta OtherActor))
  (if (not (Variables|/Game/Running_game/Blueprints/Character/BP_PlayerSanta.BP_PlayerSanta_C|GetIsSmall _asbp_player_santa))
    (Default|Death _asbp_player_santa)
    (Utilities|FlowControl|Delay 1.0)
    (Game|SetGamePaused true)))

(event EventTick
  (params (DeltaSeconds :type Float%20%28single-precision%29))
  (|CallParentFunction DeltaSeconds) ; 지금 이 노드는 비활성 상태입니다. \n핀을 끌어서 다른 노드를 연결하면 활성화됩니다.
)

(fn ConstructionScript
  (|CallParentFunction))