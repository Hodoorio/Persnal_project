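; BP_Car2 is a car obstacle in the running game that drives along X when the Santa player approaches and calls PlayerDie on collision overlaps.
; PlayerCatchSensor starts the TL_Move timeline, which lerps the mesh's X toward an Arrow component's position while keeping Y and Z.
; The lerp starts from the mesh's current position each update, so movement compounds rather than following the curve directly.
; The actor destroys itself after a short delay once the timeline finishes.
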(event OnComponentBeginOverlap(CarCollision)
  (params (OverlappedComponent :type Primitive%20Component%20Object%20Reference) (OtherActor :type Actor%20Object%20Reference) (OtherComp :type Primitive%20Component%20Object%20Reference) (OtherBodyIndex :type Integer) (bFromSweep :type Boolean) (SweepResult :type Hit%20Result%20Structure%20%28by%20ref%29))
  (CallFunction|PlayerDie OtherActor))

(event OnComponentBeginOverlap(PlayerCatchSensor)
  (params (OverlappedComponent :type Primitive%20Component%20Object%20Reference) (OtherActor :type Actor%20Object%20Reference) (OtherComp :type Primitive%20Component%20Object%20Reference) (OtherBodyIndex :type Integer) (bFromSweep :type Boolean) (SweepResult :type Hit%20Result%20Structure%20%28by%20ref%29))
  (bind _staticmesh (Variables|Default|GetStaticMesh))
  (bind _returnvalue (Transformation|GetWorldLocation _staticmesh))
  (bind (_x _y _z) (Math|Vector|BreakVector _returnvalue))
  (Utilities|Casting|CastToBP_PlayerSanta OtherActor)
  (bind _move_obstacle (Timeline|TL_Move PlayFromStart)
    (:Update
      (Transformation|SetWorldLocation _staticmesh (Math|Vector|MakeVector (Math|Float|Lerp _x (.X (Math|Vector|BreakVector (Transformation|GetWorldLocation (Variables|Default|GetArrow)))) _move_obstacle) _y _z) false false))
    (:Finished
      (Utilities|FlowControl|Delay 5.0)
      (Actor|DestroyActor))))

(event EventBeginPlay
  (|CallParentFunction) ; 지금 이 노드는 비활성 상태입니다. \n핀을 끌어서 다른 노드를 연결하면 활성화됩니다.
)

(event Collision|EventActorBeginOverlap
  (params (OtherActor :type Actor%20Object%20Reference))
  (|CallParentFunction OtherActor) ; 지금 이 노드는 비활성 상태입니다. \n핀을 끌어서 다른 노드를 연결하면 활성화됩니다.
)

(event EventTick
  (params (DeltaSeconds :type Float%20%28single-precision%29))
  (|CallParentFunction DeltaSeconds) ; 지금 이 노드는 비활성 상태입니다. \n핀을 끌어서 다른 노드를 연결하면 활성화됩니다.
)

(fn ConstructionScript
  (|CallParentFunction))