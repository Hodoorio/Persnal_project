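; Player Santa character for a three-lane endless runner, auto-running forward once W is pressed.
; Possession sets up HUD, Enhanced Input and a looping GameMode AddPortal timer.
; Input drives jumping, speed and shrink toggles, and timeline-lerped lane changes, while overlapping "Speed"-tagged actors multiplies both run speeds.
; Death ragdolls the mesh, shows game-over UI and saves GameMode high score and cookies to separate save slots.
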(event OnComponentBeginOverlap(Box)
  (params (OverlappedComponent :type Primitive%20Component%20Object%20Reference) (OtherActor :type Actor%20Object%20Reference) (OtherComp :type Primitive%20Component%20Object%20Reference) (OtherBodyIndex :type Integer) (bFromSweep :type Boolean) (SweepResult :type Hit%20Result%20Structure%20%28by%20ref%29))
  ;[0.15 0.15 0.15 0.5] Speed 태그 floor일 경우 기본 속도와 Interval 속도 증가(SecondStage 용)
  (if (Actor|ActorHasTag OtherActor "Speed")
    (Variables|Default|SetDefaultSpeed (* (Variables|Default|GetDefaultSpeed) 1.2))
    (Variables|Default|SetIntervalSpeed (* (Variables|Default|GetIntervalSpeed) 1.2))))

(event Custom|ChangeLanes
  (params (shiftLanes :type Integer))
  (bind _returnvalue (Transformation|GetActorLocation))
  (bind (_x _y _z) (Math|Vector|BreakVector _returnvalue))
  ;[0.15 0.15 0.15 0.5] 레인 변경
  (Variables|Default|SetTargetLaneIndex (Math|Integer|Clamp(Integer) (+ shiftLanes (Variables|Default|GetCurrentLaneIndex)) 0 2))
  (Variables|Default|SetCurrentYPosition (.Y (Math|Vector|BreakVector (Transformation|GetActorLocation))))
  (bind _changelanes (Timeline|Transition PlayFromStart)
    (:Update
      (Transformation|SetActorLocation (Math|Vector|MakeVector _x (Math|Float|Lerp (Variables|Default|GetCurrentYPosition) (Utilities|Array|Get(acopy) (Variables|Default|GetLanePosition) (Variables|Default|GetTargetLaneIndex)) _changelanes) _z) false false))
    (:Finished
      (Variables|Default|SetCurrentLaneIndex (Variables|Default|GetTargetLaneIndex)))))

(event Input|EnhancedActionEvents|EnhancedInputActionIA_PlayerLeft
  (params (ActionValue :type Boolean) (ElapsedSeconds :type Float%20%28double-precision%29) (TriggeredSeconds :type Float%20%28double-precision%29) (InputAction :type Input%20Action%20Object%20Reference :default "/Game/Running_game/Input/IA_PlayerLeft.IA_PlayerLeft"))
  ;[0.15 0.15 0.15 0.5] 레인 변경
  (CallFunction|ChangeLanes -1))

(event Input|EnhancedActionEvents|EnhancedInputActionIA_PlayerRight
  (params (ActionValue :type Boolean) (ElapsedSeconds :type Float%20%28double-precision%29) (TriggeredSeconds :type Float%20%28double-precision%29) (InputAction :type Input%20Action%20Object%20Reference :default "/Game/Running_game/Input/IA_PlayerRight.IA_PlayerRight"))
  ;[0.15 0.15 0.15 0.5] 레인 변경
  (CallFunction|ChangeLanes 1))

(event Input|EnhancedActionEvents|EnhancedInputActionIA_PlayerJump
  (params (ActionValue :type Boolean) (ElapsedSeconds :type Float%20%28double-precision%29) (TriggeredSeconds :type Float%20%28double-precision%29) (InputAction :type Input%20Action%20Object%20Reference :default "/Game/Running_game/Input/IA_PlayerJump.IA_PlayerJump"))
  ;[0.15 0.15 0.15 0.5] 점프와 빨리 달리기
  (:Started
    (switch Utilities|FlowControl|Switch|SwitchonEMovementMode (Variables|/Script/Engine.CharacterMovementComponent|GetMovementMode (Variables|Character|GetCharacterMovement))
      (:MOVE_Walking
        (Character|Jump))))
  (:Completed
    (Character|StopJumping)))

(event Input|EnhancedActionEvents|EnhancedInputActionIA_PlayerInterval
  (params (ActionValue :type Boolean) (ElapsedSeconds :type Float%20%28double-precision%29) (TriggeredSeconds :type Float%20%28double-precision%29) (InputAction :type Input%20Action%20Object%20Reference :default "/Game/Running_game/Input/IA_PlayerInterval.IA_PlayerInterval"))
  ;[0.15 0.15 0.15 0.5] 점프와 빨리 달리기
  (:Started
    (bind _output_get (Variables|Default|SetIsInterval (not (Variables|Default|GetIsInterval))))
    (if _output_get
      (Variables|/Script/Engine.CharacterMovementComponent|SetMaxWalkSpeed (Variables|Character|GetCharacterMovement) (Variables|Default|GetIntervalSpeed))
      (else
        (Variables|/Script/Engine.CharacterMovementComponent|SetMaxWalkSpeed (Variables|Character|GetCharacterMovement) (Variables|Default|GetDefaultSpeed))))))

(event Input|EnhancedActionEvents|EnhancedInputActionIA_PlayerSmall
  (params (ActionValue :type Boolean) (ElapsedSeconds :type Float%20%28double-precision%29) (TriggeredSeconds :type Float%20%28double-precision%29) (InputAction :type Input%20Action%20Object%20Reference :default "/Game/Running_game/Input/IA_PlayerSmall.IA_PlayerSmall"))
  ;[0.15 0.15 0.15 0.5] 웅크리기 처리(캐릭터 스케일 조정)
  (:Started
    (bind _output_get (Variables|Default|SetIsSmall (not (Variables|Default|GetIsSmall))))
    (bind _alpha (Timeline|TL_Lerp PlayFromStart)
      (:Update
        (if _output_get
          (Transformation|SetActorScale3D (Math|Vector|Lerp(Vector) (Variables|Default|GetSmallScale) (Transformation|GetActorScale3D) _alpha))
          (Variables|/Script/Engine.CharacterMovementComponent|SetAirControl (Variables|Character|GetCharacterMovement) 1e+01)
          (else
            (Transformation|SetActorScale3D (Math|Vector|Lerp(Vector) (Variables|Default|GetDefaultScale) (Transformation|GetActorScale3D) _alpha))))))))

(event EventPossessed
  (params (NewController :type Controller%20Object%20Reference))
  (bind _returnvalue (Game|GetPlayerController 0))
  ;[0.15 0.15 0.15 0.5] 캐릭터에 빙의 되었을때 UI를 생성하고 입력 컨텍스트를 연결
  (if (== NewController _returnvalue)
    (Input|SetInputModeGameOnly _returnvalue false)
    (bind _returnvalue_2 (UserInterface|CreateWidget "/Game/Running_game/Blueprints/HUD/Gameplay_UI.Gameplay_UI_C"))
    (UserInterface|Viewport|AddtoViewport _returnvalue_2 0)
    (Input|AddMappingContext (PlayerController|LocalPlayerSubsystems|GetEnhancedInputLocalPlayerSubsystem _returnvalue) "/Game/Running_game/Input/IMC_Runner.IMC_Runner" 0 "(bIgnoreAllPressedKeysUntilRelease=True,bForceImmediately=False,bNotifyUserSettings=False)")
    (Utilities|Time|SetTimerbyFunctionName (Game|GetGameMode) "AddPortal" (Variables|Default|GetPortalSpawnTime) true)))

(event EventTick
  (params (DeltaSeconds :type Float%20%28single-precision%29))
  ;[0.15 0.15 0.15 0.5] 무한히 앞으로 달리기
  (if (Variables|Default|Getrun)
    (Pawn|Input|AddMovementInput (Math|Vector|GetForwardVector (Math|Rotator|MakeRotator 0.0 0.0 (.yaw (Pawn|GetControlRotation :!class /Script/Engine.Pawn)))) 1.0 false)))

(event Input|KeyboardEvents|W
  (params (Key :type Key%20Structure :default "None"))
  (:Pressed
    (Variables|Default|Setrun true)))

(fn ConstructionScript)

(fn Death
  (bind _returnvalue (Game|GetPlayerController 0))
  ;[0.15 0.15 0.15 0.5] 죽었을때를 처리
  (Pawn|Components|CharacterMovement|DisableMovement (Variables|Character|GetCharacterMovement))
  (Input|DisableInput 0)
  (Physics|SetSimulatePhysics (Variables|Character|GetMesh) true)
  (Viewport|RemoveAllWidgets)
  (bind _returnvalue_2 (UserInterface|CreateWidget "/Game/Running_game/Blueprints/HUD/GameOver_UI.GameOver_UI_C"))
  (UserInterface|Viewport|AddtoViewport _returnvalue_2 0)
  (Input|SetInputModeUIOnly _returnvalue 0 "DoNotLock" false)
  (Variables|/Script/Engine.PlayerController|SetbShowMouseCursor _returnvalue true)
  (CallFunction|SaveHighScore)
  (CallFunction|UpdateCoins))

(fn SaveHighScore
  (bind _asgm_run_santa (Utilities|Casting|CastToGM_RunSanta (Game|GetGameMode)))
  (bind _returnvalue (SaveGame|DoesSaveGameExist "HighScoreValue"))
  (if _returnvalue
    (bind _returnvalue_2 (SaveGame|LoadGamefromSlot "HighScoreValue"))
    (bind _output_get (Variables|Default|SetSaverSubClass _returnvalue_2))
    (bind _assanta_save_game (Utilities|Casting|CastToSanta_SaveGame _output_get))
    (if (> (Variables|/Game/Running_game/Blueprints/Framework/GM_RunSanta.GM_RunSanta_C|GetCurrentPoints _asgm_run_santa) (Variables|/Game/Running_game/Blueprints/Framework/Santa_SaveGame.Santa_SaveGame_C|GetHighScoreValue _assanta_save_game))
      (Variables|/Game/Running_game/Blueprints/Framework/Santa_SaveGame.Santa_SaveGame_C|SetHighScoreValue _assanta_save_game (Variables|/Game/Running_game/Blueprints/Framework/GM_RunSanta.GM_RunSanta_C|GetCurrentPoints _asgm_run_santa))
      (SaveGame|SaveGametoSlot (Variables|Default|GetSaverSubClass) "HighScoreValue"))
    (else
      (bind _returnvalue_3 (SaveGame|CreateSaveGameObject "/Game/Running_game/Blueprints/Framework/Santa_SaveGame.Santa_SaveGame_C"))
      (bind _output_get_2 (Variables|Default|SetSaverSubClass _returnvalue_3))
      (bind _assanta_save_game_2 (Utilities|Casting|CastToSanta_SaveGame _output_get_2))
      (Variables|/Game/Running_game/Blueprints/Framework/Santa_SaveGame.Santa_SaveGame_C|SetHighScoreValue _assanta_save_game_2 (Variables|/Game/Running_game/Blueprints/Framework/GM_RunSanta.GM_RunSanta_C|GetCurrentPoints _asgm_run_santa))
      (SaveGame|SaveGametoSlot (Variables|Default|GetSaverSubClass) "HighScoreValue"))))

(fn UpdateCoins
  (bind _asgm_run_santa (Utilities|Casting|CastToGM_RunSanta (Game|GetGameMode)))
  (bind _returnvalue (SaveGame|DoesSaveGameExist "CookieValue"))
  (if _returnvalue
    (bind _returnvalue_2 (SaveGame|LoadGamefromSlot "CookieValue"))
    (bind _output_get (Variables|Default|SetSaverSubClass _returnvalue_2))
    (bind _assanta_save_game (Utilities|Casting|CastToSanta_SaveGame _output_get))
    (Variables|/Game/Running_game/Blueprints/Framework/Santa_SaveGame.Santa_SaveGame_C|SetCookieValue _assanta_save_game (Variables|/Game/Running_game/Blueprints/Framework/GM_RunSanta.GM_RunSanta_C|GetCookies _asgm_run_santa))
    (SaveGame|SaveGametoSlot (Variables|Default|GetSaverSubClass) "CookieValue")
    (else
      (bind _returnvalue_3 (SaveGame|CreateSaveGameObject "/Game/Running_game/Blueprints/Framework/Santa_SaveGame.Santa_SaveGame_C"))
      (bind _output_get_2 (Variables|Default|SetSaverSubClass _returnvalue_3))
      (bind _assanta_save_game_2 (Utilities|Casting|CastToSanta_SaveGame _output_get_2))
      (Variables|/Game/Running_game/Blueprints/Framework/Santa_SaveGame.Santa_SaveGame_C|SetCookieValue _assanta_save_game_2 (Variables|/Game/Running_game/Blueprints/Framework/GM_RunSanta.GM_RunSanta_C|GetCookies _asgm_run_santa))
      (SaveGame|SaveGametoSlot (Variables|Default|GetSaverSubClass) "CookieValue"))))

(fn GetIsInterval
  (return (Variables|Default|GetIsInterval)))

(fn GetIsSmall
  (return (Variables|Default|GetIsSmall)))