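; BP_Cookie is a collectible cookie for the Santa running game.
; On overlap with BP_PlayerSanta, it increments the Cookies count in GM_RunSanta, prints the total, destroys itself and calls the player's UpdateCoins.
; A second sequence branch destroys the cookie when it overlaps a BP_Obstacles_Wall.
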(event Collision|EventActorBeginOverlap
  (params (OtherActor :type Actor%20Object%20Reference))
  (Utilities|FlowControl|Sequence
    (:then_0
      (bind _asbp_player_santa (Utilities|Casting|CastToBP_PlayerSanta OtherActor))
      (bind _asgm_run_santa (Utilities|Casting|CastToGM_RunSanta (Game|GetGameMode)))
      (bind _result (Math|Integer|IncrementInt (Variables|/Game/Running_game/Blueprints/Framework/GM_RunSanta.GM_RunSanta_C|GetCookies _asgm_run_santa))
        (:%20%20
          (Development|PrintString (Utilities|String|ToString(Integer) _result) true true "(R=0.000000,G=1.000000,B=0.019322,A=1.000000)")
          (Actor|DestroyActor)
          (Default|UpdateCoins _asbp_player_santa))))
    (:then_1
      (Utilities|Casting|CastToBP_Obstacles_Wall OtherActor)
      (Actor|DestroyActor))))

(event EventTick
  (params (DeltaSeconds :type Float%20%28single-precision%29)))

(fn ConstructionScript)